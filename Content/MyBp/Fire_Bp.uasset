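; Fire hazard actor that starts with its fire effect and audio switched off.
; On BeginPlay it binds to the FireStart dispatcher on a referenced object, which activates both and prints a message when fired.
; The Box overlap prints a red death message for the player's SunWukong character, whether or not the fire is active.
; Player destruction and level reload are left unconnected, so the hazard does not actually kill.
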(event OnComponentBeginOverlap(Box)
  (params (OverlappedComponent :type Primitive%20Component%20Object%20Reference) (OtherActor :type Actor%20Object%20Reference) (OtherComp :type Primitive%20Component%20Object%20Reference) (OtherBodyIndex :type Integer) (bFromSweep :type Boolean) (SweepResult :type Hit%20Result%20Structure%20%28by%20ref%29))
  (bind _assun_wukong_player_character (Utilities|Casting|CastToSunWukongPlayerCharacter OtherActor))
  (if (== _assun_wukong_player_character (Game|GetPlayerCharacter 0))
    (Development|PrintString "你被烧死了哈哈哈" true true "(R=0.947917,G=0.069119,B=0.069119,A=1.000000)")))

(event Custom|CustomEvent_0
  (Development|PrintString "这是熊熊燃烧的大火")
  (Components|Activation|SetActive (Variables|Default|GetP_Fire) true false)
  (Components|Activation|SetActive (Variables|Default|GetFire%20Audio) true false))

(event EventBeginPlay
  (Components|Activation|SetActive (Variables|Default|GetP_Fire) false false)
  (Components|Activation|SetActive (Variables|Default|GetFire%20Audio) false false)
  (EventDispatchers|AssignFireStart (Variables|Default|GetNewVar_0) (delegate Custom|CustomEvent_0)))

(event Collision|EventActorBeginOverlap
  (params (OtherActor :type Actor%20Object%20Reference)))

(event EventTick
  (params (DeltaSeconds :type Float%20%28single-precision%29)))

(fn ConstructionScript
  (|CallParentFunction))